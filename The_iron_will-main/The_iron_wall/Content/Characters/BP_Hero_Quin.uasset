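; BP_Hero_Quin is a playable hero character with movement, look, weapon fire and aim-down-sights input.
; Axis inputs drive movement along actor forward and right vectors plus controller yaw and pitch.
; Firing spawns an attached emitter, plays a 2D sound and runs a debug-drawn Visibility trace from the Muzzle socket, with the hit unused.
; ADS sets IsADS locally, and remote instances also forward it through a server event.
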(event Custom|Svr_SetlsAds
  (params (IsADS :type Boolean))
  (Variables|Default|SetIsADS IsADS))

(event Input|ActionEvents|InputActionADS
  (params (Key :type Key%20Structure :default "None"))
  (:Pressed
    (Networking|SwitchHasAuthority
      (:Authority
        _)
      (:Remote
        (CallFunction|SvrSetlsAds true)))
    (Variables|Default|SetIsADS true))
  (:Released
    (Networking|SwitchHasAuthority
      (:Authority
        _)
      (:Remote
        (CallFunction|SvrSetlsAds false)))
    (Variables|Default|SetIsADS false)))

(event Input|ActionEvents|InputActionFireWeapon
  (params (Key :type Key%20Structure :default "None"))
  (bind _weaponmesh (Variables|Default|GetWeaponMesh))
  (bind _returnvalue (Transformation|GetSocketTransform _weaponmesh "Muzzle" "RTS_World"))
  (:Pressed
    (Effects|SpawnEmitterAttached 0 (Variables|Default|GetWeaponMesh) "None")
    (Audio|PlaySound2D "/Engine/VREditor/Sounds/VR_grab_Cue.VR_grab_Cue" 1.0 1.0 0.0 0 0)
    (Collision|LineTraceByChannel (.location _returnvalue) (+ (.location _returnvalue) (* (Math|Vector|GetForwardVector (.rotation _returnvalue)) 10000)) "TraceTypeQuery1" false 0 "ForDuration")))

(event Input|AxisEvents|InputAxisMoveForward
  (params (AxisValue :type Float%20%28single-precision%29))
  (Pawn|Input|AddMovementInput (Transformation|GetActorForwardVector) AxisValue false))

(event Input|AxisEvents|InputAxisMoveRight
  (params (AxisValue :type Float%20%28single-precision%29))
  (Pawn|Input|AddMovementInput (Transformation|GetActorRightVector) AxisValue false))

(event Input|AxisEvents|InputAxisTurn
  (params (AxisValue :type Float%20%28single-precision%29))
  (Pawn|Input|AddControllerYawInput AxisValue))

(event Input|AxisEvents|InputAxisLookUp
  (params (AxisValue :type Float%20%28single-precision%29))
  (Pawn|Input|AddControllerPitchInput AxisValue))

(fn ConstructionScript)